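; Player character that handles Enhanced Input movement, look, jump, run, interaction and melee attacks, and adds a dialogue widget on BeginPlay.
; Interact messages the first overlapping actor implementing BPI_Interact.
; Attack plays a montage chosen by AttackIndex, gated by CanAttack, with both reset on completion.
; HitDetection, not called here, sphere-traces pawns at the matching hand or foot socket and sends DetectDamageMessage on initial overlap.
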(event `self.ReceiveBeginPlay`
  (bind _returnvalue (subsystem `EnhancedInputLocalPlayerSubsystem`))
  (`/Engine/EditorBlueprintResources/StandardMacros.IsValid` _returnvalue
    (:`Is Valid`
      (`EnhancedInputSubsystemInterface.AddMappingContext` _returnvalue "/Game/02_Blueprints/01_Player/01_Inputs/IMC_Player.IMC_Player" 0 (struct))
      (bind _returnvalue_2 (`|CreateWidget` "/Game/03_UI/WB_Dialogue.WB_Dialogue_C"))
      (bind _output_get (set `self.UIRef` _returnvalue_2))
      (`UserWidget.AddToViewport` _output_get 0))))

(event `EnhancedInput|/Game/02_Blueprints/01_Player/01_Inputs/IA_Jump`
  (params (ActionValue :type Boolean) (ElapsedSeconds :type "Float (double-precision)") (TriggeredSeconds :type "Float (double-precision)") (InputAction :type "InputAction Object Reference" :default "/Game/02_Blueprints/01_Player/01_Inputs/IA_Jump.IA_Jump"))
  (:`Triggered`
    (`self.Jump`)))

(event `EnhancedInput|/Game/02_Blueprints/01_Player/01_Inputs/IA_Move`
  (params (ActionValue :type "Vector2D Structure") (ElapsedSeconds :type "Float (double-precision)") (TriggeredSeconds :type "Float (double-precision)") (InputAction :type "InputAction Object Reference" :default "/Game/02_Blueprints/01_Player/01_Inputs/IA_Move.IA_Move"))
  (bind (_returnvalue_roll _returnvalue_pitch _returnvalue_yaw) (`KismetMathLibrary.BreakRotator` (`self.GetControlRotation`)))
  (bind (_returnvalue_roll_2 _returnvalue_pitch_2 _returnvalue_yaw_2) (`KismetMathLibrary.BreakRotator` (`self.GetControlRotation`)))
  (:`Triggered`
    (`self.AddMovementInput` (`KismetMathLibrary.GetForwardVector` (`KismetMathLibrary.MakeRotator` 0.0 0.0 _returnvalue_yaw_2)) ActionValue_Y)
    (`self.AddMovementInput` (`KismetMathLibrary.GetRightVector` (`KismetMathLibrary.MakeRotator` 0.0 0.0 _returnvalue_yaw)) ActionValue_X)))

(event `EnhancedInput|/Game/02_Blueprints/01_Player/01_Inputs/IA_Look`
  (params (ActionValue :type "Vector2D Structure") (ElapsedSeconds :type "Float (double-precision)") (TriggeredSeconds :type "Float (double-precision)") (InputAction :type "InputAction Object Reference" :default "/Game/02_Blueprints/01_Player/01_Inputs/IA_Look.IA_Look"))
  (:`Triggered`
    (`self.AddControllerYawInput` ActionValue_X)
    (`self.AddControllerPitchInput` ActionValue_Y)))

(event `EnhancedInput|/Game/02_Blueprints/01_Player/01_Inputs/IA_Interact`
  (params (ActionValue :type Boolean) (ElapsedSeconds :type "Float (double-precision)") (TriggeredSeconds :type "Float (double-precision)") (InputAction :type "InputAction Object Reference" :default "/Game/02_Blueprints/01_Player/01_Inputs/IA_Interact.IA_Interact"))
  (:`Triggered`
    (for _array_element (`self.GetOverlappingActors` null)
      (if (`KismetSystemLibrary.DoesImplementInterface` _array_element "/Game/02_Blueprints/01_Player/BPI_Interact.BPI_Interact_C")
        (message `/Game/02_Blueprints/01_Player/BPI_Interact.Interact` _array_element)
        (break)))))

(event `EnhancedInput|/Game/02_Blueprints/01_Player/01_Inputs/IA_Run`
  (params (ActionValue :type Boolean) (ElapsedSeconds :type "Float (double-precision)") (TriggeredSeconds :type "Float (double-precision)") (InputAction :type "InputAction Object Reference" :default "/Game/02_Blueprints/01_Player/01_Inputs/IA_Run.IA_Run"))
  (bind _charactermovement (`self.CharacterMovement`))
  (:`Triggered`
    (set `CharacterMovementComponent.MaxWalkSpeed` 1200.0 _charactermovement))
  (:`Canceled`
    (set `CharacterMovementComponent.MaxWalkSpeed` 600.0 _charactermovement :!label _label))
  (:`Completed`
    (goto _label)))

(event `EnhancedInput|/Game/02_Blueprints/01_Player/01_Inputs/IA_Attack`
  (params (ActionValue :type Boolean) (ElapsedSeconds :type "Float (double-precision)") (TriggeredSeconds :type "Float (double-precision)") (InputAction :type "InputAction Object Reference" :default "/Game/02_Blueprints/01_Player/01_Inputs/IA_Attack.IA_Attack"))
  (:`Triggered`
    (`self.canAttack`
      (:`then`
        (set `self.canAttack` false)
        (`|PlayMontage` (`self.Mesh`) (select `int` (`self.AttackIndex`) :`0` "/Game/04_Assets/02_Animations/01_Fist_Fight_A_Montage.01_Fist_Fight_A_Montage" :`1` "/Game/04_Assets/02_Animations/02_Chapa_2_Montage.02_Chapa_2_Montage" :`2` "/Game/04_Assets/02_Animations/03_Inside_Crescent_Kick_Montage.03_Inside_Crescent_Kick_Montage" :!type "AnimMontage Object Reference")
          (:`then`
            (`/Engine/EditorBlueprintResources/StandardMacros.IncrementInt` (`self.AttackIndex`)))
          (:`OnCompleted`
            (set `self.canAttack` true)
            (set `self.AttackIndex` 0))))
      (:`else`))))

(fn `HitDetection`
  (bind _returnvalue (`SceneComponent.GetSocketLocation` (`self.Mesh`) (select `int` (`self.AttackIndex`) :`0` "LeftHand" :`1` "LeftHand" :`2` "RightFoot" :`3` "RightFoot" :!type "Name")))
  (bind _outhit (`KismetSystemLibrary.SphereTraceSingleForObjects` :`Start` _returnvalue :`End` _returnvalue :`Radius` 20.0 :`ObjectTypes` (`|MakeArray` "ObjectTypeQuery3" :!type "EObjectTypeQuery Enum") :`DrawDebugType` "ForDuration"))
  (bind (_bblockinghit _binitialoverlap _time _distance _location _impactpoint _normal _impactnormal _physmat _hitactor) (`GameplayStatics.BreakHitResult` _outhit))
  (if _binitialoverlap
    (message `/Game/02_Blueprints/01_Player/BPI_Damage_Detection.Detect Damage` _hitactor)))

(fn `UserConstructionScript`)