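; BP_Enemy1 is a test enemy that tracks hit points and dies when they run out.
; It sets its HP on BeginPlay, and its DetectDamage event subtracts the incoming damage from that value.
; At zero or below the actor destroys itself; otherwise it prints the remaining HP as text.
; Overlap, Tick and the construction script do nothing.
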(event `self.ReceiveBeginPlay`
  (set `self.HP` 1000))

(event `/Game/02_Blueprints/01_Player/BPI_Damage_Detection.Detect Damage`
  (params (Damage :type Integer))
  (bind _output_get (set `self.HP` (- (`self.HP`) Damage)))
  (if (<= _output_get 0)
    (`self.K2_DestroyActor`)
    (else
      (`KismetSystemLibrary.PrintText` (`KismetTextLibrary.Conv_StringToText` (`KismetStringLibrary.Conv_IntToString` (`self.HP`)))))))

(fn `UserConstructionScript`)