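; BP_Cube is an interactable test object that steps through an array of dialogue lines, one per Interact event.
; Shortly after BeginPlay it copies the player pawn's UIRef.
; Interact creates a WB_Dialogue widget if that reference is invalid, sets the next line, and after the last removes the widget and resets the index.
; Overlap events are empty, and unconnected nodes hold a start/end dialogue toggle and sound playback.
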(event `self.ReceiveBeginPlay`
  (`KismetSystemLibrary.Delay` 0.1)
  (bind _asbp_player (cast `/Game/02_Blueprints/01_Player/BP_Player` (`GameplayStatics.GetPlayerPawn` 0)))
  (set `self.UIRef` (`/Game/02_Blueprints/01_Player/BP_Player.UIRef` _asbp_player)))

(event `/Game/02_Blueprints/01_Player/BPI_Interact.Interact`
  (if (< (`self.dialogueIndex`) (`KismetArrayLibrary.Array_Length` (`self.Dialogue`)))
    (`self.UIRef`
      (:`then`
        _)
      (:`else`
        (bind _returnvalue (`|CreateWidget` "/Game/03_UI/WB_Dialogue.WB_Dialogue_C" (`GameplayStatics.GetPlayerController` 0)))
        (bind _output_get (set `self.UIRef` _returnvalue))
        (`UserWidget.AddToViewport` _output_get 0)))
    (`TextBlock.SetText` (`/Game/03_UI/WB_Dialogue.TextBlock_0` (`self.UIRef`)) (`KismetTextLibrary.Conv_StringToText` (`|GetArrayItem` (`self.Dialogue`) (`self.dialogueIndex`))))
    (`/Engine/EditorBlueprintResources/StandardMacros.IncrementInt` (`self.dialogueIndex`))
    (else
      (`Widget.RemoveFromParent` (`self.UIRef`))
      (set `self.UIRef` null)
      (set `self.dialogueIndex` 0))))

(event `self.Box.OnComponentEndOverlap`
  (params (OverlappedComponent :type "PrimitiveComponent Object Reference") (OtherActor :type "Actor Object Reference") (OtherComp :type "PrimitiveComponent Object Reference") (OtherBodyIndex :type Integer)))

(fn `UserConstructionScript`)